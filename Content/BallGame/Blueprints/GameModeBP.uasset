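; Game mode Blueprint for BallGame that provides functions to pause and unpause the game.
; PauseGame halts play, shows the Menu widget and switches to Game and UI input with the mouse cursor visible.
; UnpauseGame resumes play, clears all widgets, re-adds the UI widget and restores game-only input with the cursor hidden.
; Both functions create their widget only when the stored reference is invalid, then reuse it.
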(fn ConstructionScript)

(fn PauseGame
  (Game|SetGamePaused true)
  (Utilities|IsValid (Variables|Default|GetMenu)
    (:Is%20Valid
      _)
    (:Is%20Not%20Valid
      (bind _returnvalue (UserInterface|CreateWidget "/Game/BallGame/Blueprints/Menu.Menu_C" (Game|GetPlayerController 0)))
      (Variables|Default|SetMenu _returnvalue)))
  (UserInterface|Viewport|AddtoViewport (Variables|Default|GetMenu) 0)
  (Input|SetInputModeGameandUI (Game|GetPlayerController 0) (Variables|Default|GetMenu) "DoNotLock" true)
  (Variables|/Script/Engine.PlayerController|SetbShowMouseCursor (Game|GetPlayerController 0) true))

(fn UnpauseGame
  (bind _returnvalue (Game|GetPlayerController 0))
  (Game|SetGamePaused false)
  (Viewport|RemoveAllWidgets)
  (Utilities|IsValid (Variables|Default|GetUI)
    (:Is%20Valid
      _)
    (:Is%20Not%20Valid
      (bind _returnvalue_2 (UserInterface|CreateWidget "/Game/BallGame/Blueprints/UI.UI_C" (Game|GetPlayerController 0)))
      (Variables|Default|SetUI _returnvalue_2)))
  (UserInterface|Viewport|AddtoViewport (Variables|Default|GetUI) 0)
  (Input|SetInputModeGameOnly _returnvalue)
  (Variables|/Script/Engine.PlayerController|SetbShowMouseCursor _returnvalue false))