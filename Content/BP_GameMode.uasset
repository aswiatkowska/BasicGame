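; Game mode Blueprint that tracks collected pickup points and handles the win condition for a simple collection game.
; BeginPlay creates the UserInterface widget and resets the score.
; UpdatePoints increments the score, pushes it to the widget and calls EndGame, which at four or more points shows the win message and loads NewMap after a short delay.
; The node that hides the win message is disconnected and never runs.
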(event Custom|ResetGame
  ;[1 1 1] Reset points and turn off the win message
  (Variables|Default|SetcurrentPoints 0)
  (Variables|/Game/UserInterface.UserInterface_C|SetPoint (Variables|Default|GetcurrentUI) 0))

(event Custom|EndGame
  ;[1 1 1] Check to see if all the pickups got collected and restart the game
  (if (>= (Variables|Default|GetcurrentPoints) 4)
    (Variables|/Game/UserInterface.UserInterface_C|SetyouWinOpacity (Variables|Default|GetcurrentUI) 1.0)
    (Utilities|FlowControl|Delay 1.0)
    (Game|OpenLevel(byName) "NewMap")))

(event Custom|UpdatePoints
  ;[1 1 1] Increment points by 1 and  update the UI
  (bind _output_get (Variables|Default|SetcurrentPoints (+ 1 (Variables|Default|GetcurrentPoints))))
  (Variables|/Game/UserInterface.UserInterface_C|SetPoint (Variables|Default|GetcurrentUI) _output_get)
  (CallFunction|EndGame))

(event EventBeginPlay
  ;[1 1 1] New instance of UI added to the screen
  (bind _returnvalue (UserInterface|CreateWidget "/Game/UserInterface.UserInterface_C"))
  (bind _output_get (Variables|Default|SetcurrentUI _returnvalue))
  (UserInterface|Viewport|AddtoViewport _output_get 0)
  (CallFunction|ResetGame))

(fn ConstructionScript)